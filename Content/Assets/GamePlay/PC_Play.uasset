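; PC_Play is the gameplay player controller, handling backpack UI and interaction with BP_Build actors.
; OpenBP sends the open build, or one hit by a camera trace, to a server event calling its FUNTrace; a trace miss toggles the backpack.
; A client event stores OpenActor and switches backpack visibility, input mode and cursor.
; Number keys add resources by ID through PlayerState, to the player or an open BP_Build_BaoXiang chest.
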(event `EVE_Client_OpenBp`
  (params (Build :type "/Game/Assets/Build/BP_Build Object Reference") (Open :type Boolean))
  ;[0 0.8124 1] client
  (set `self.OpenActor` Build)
  (`self.FUN_OpenBp` Open))

(event `EVE_Server_Build_Trace`
  (params (Build :type "/Game/Assets/Build/BP_Build Object Reference") (PC :type "/Game/Assets/GamePlay/PC_Play Object Reference"))
  ;[1 0 0.9286] Server build交互
  (`/Game/Assets/Build/BP_Build_BaoXiang.FUN_Trace` Build PC))

(event `Key|One`
  (params (Key :type "Key Structure"))
  (:`Pressed`
    (`/Game/Assets/GamePlay/PS_Play.EVE_Server_Add_Rs_ByID` (`/Game/Assets/GamePlay/FUNL_Play.FUNL_GetPlayerState`) "1")))

(event `Key|Two`
  (params (Key :type "Key Structure"))
  (:`Pressed`
    (`/Game/Assets/GamePlay/PS_Play.EVE_Server_Add_Rs_ByID` (`/Game/Assets/GamePlay/FUNL_Play.FUNL_GetPlayerState`) "2")))

(event `InputAction|OpenBP`
  (params (Key :type "Key Structure"))
  (bind _returnvalue (`GameplayStatics.GetPlayerCameraManager` 0))
  (bind _returnvalue_2 (`PlayerCameraManager.GetCameraLocation` _returnvalue))
  ;[1 1 1] 打开关闭背包
  (:`Pressed`
    (`/Engine/EditorBlueprintResources/StandardMacros.IsValid` (`self.OpenActor`)
      (:`Is Valid`
        (`self.EVE_Server_Build_Trace` (`self.OpenActor`) self))
      (:`Is Not Valid`
        (bind (_outhit _returnvalue_3) (`KismetSystemLibrary.LineTraceSingle` _returnvalue_2 (+ _returnvalue_2 (* (`self.GetActorForwardVector` _returnvalue) 1000.0)) "TraceTypeQuery1" true (`|MakeArray` (`GameplayStatics.GetPlayerCharacter` 0) :!type "Actor Object Reference") "ForDuration"))
        (if _returnvalue_3
          (bind _asbp_build (cast `/Game/Assets/Build/BP_Build` (`.HitActor` (`GameplayStatics.BreakHitResult` _outhit))))
          (`self.EVE_Server_Build_Trace` _asbp_build self)
          (else
            (`self.FUN_OpenBp` (not (`Widget.IsVisible` (`/Game/Assets/GamePlay/HUD_Play.UMG_BP` (`/Game/Assets/GamePlay/FUNL_Play.FUNL_GetHUD`)))))))))))

(event `Key|Three`
  (params (Key :type "Key Structure"))
  (:`Pressed`
    (`/Game/Assets/GamePlay/PS_Play.EVE_Server_Add_Rs_ByID` (`/Game/Assets/GamePlay/FUNL_Play.FUNL_GetPlayerState`) "3")))

(event `Key|Four`
  (params (Key :type "Key Structure"))
  (:`Pressed`
    (bind _asbp_build_bao_xiang (cast `/Game/Assets/Build/BP_Build_BaoXiang` (`self.OpenActor`)))
    (`/Game/Assets/GamePlay/PS_Play.EVE_Add_Rs_ToBuild` (`/Game/Assets/GamePlay/FUNL_Play.FUNL_GetPlayerState`) _asbp_build_bao_xiang "3")))

(fn `FUN_OpenBp`
  (params (Open :type Boolean))
  (bind _umg_bp (`/Game/Assets/GamePlay/HUD_Play.UMG_BP` (`/Game/Assets/GamePlay/FUNL_Play.FUNL_GetHUD`)))
  (if Open
    (`Widget.SetVisibility` _umg_bp "SelfHitTestInvisible")
    (`WidgetBlueprintLibrary.SetInputMode_GameAndUIEx` self _umg_bp)
    (set `self.bShowMouseCursor` true)
    (`/Game/Assets/UMG/UMG_BP.FUN_UpdateOpen` (`/Game/Assets/GamePlay/HUD_Play.UMG_BP` (`/Game/Assets/GamePlay/FUNL_Play.FUNL_GetHUD`)))
    (else
      (`Widget.SetVisibility` (`/Game/Assets/GamePlay/HUD_Play.UMG_BP` (`/Game/Assets/GamePlay/FUNL_Play.FUNL_GetHUD`)) "Collapsed")
      (`WidgetBlueprintLibrary.SetInputMode_GameOnly` self)
      (set `self.bShowMouseCursor` false))))

(fn `UserConstructionScript`)